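; Behavior tree task that picks the next move destination for a Dummy AI pawn.
; It fails if the Dummy can see the player.
; Otherwise it advances the LocationIndex blackboard key, wrapping at the end of the pawn's Locations array, then writes a random navigable point near the pawn to MoveToLocation and succeeds.
; The indexed Locations lookup is left unconnected, so the index does not affect the destination.
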(event EventReceiveExecuteAI
  (params (OwnerController :type AI%20Controller%20Object%20Reference) (ControlledPawn :type Pawn%20Object%20Reference))
  (bind _locationindex (Variables|Default|GetLocationIndex))
  (bind _returnvalue (Class|BTFunctionLibrary|GetBlackboardValueasInt _locationindex))
  (bind _asdummy (Utilities|Casting|CastToDummy ControlledPawn))
  (if (Variables|/Game/Character/Blueprints/Dummy.Dummy_C|GetCanSeePlayer _asdummy)
    (AI|BehaviorTree|FinishExecute false)
    (else
      (if (>= _returnvalue (- (Utilities|Array|Length (Variables|/Game/Character/Blueprints/Dummy.Dummy_C|GetLocations _asdummy)) 1))
        (Class|BTFunctionLibrary|SetBlackboardValueasInt _locationindex)
        (else
          (Class|BTFunctionLibrary|SetBlackboardValueasInt _locationindex (+ _returnvalue 1))))
      (AI|BehaviorTree|SetBlackboardValueasVector (Variables|Default|GetMoveToLocation) (.RandomLocation (Class|NavigationSystemV1|GetRandomPointinNavigableRadius (Transformation|GetActorLocation _asdummy) 5e+02 0 0)))
      (AI|BehaviorTree|FinishExecute true))))
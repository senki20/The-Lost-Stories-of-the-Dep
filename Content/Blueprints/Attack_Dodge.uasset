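; Behavior tree task that makes a Dummy AI pawn choose between attacking and dodge-rolling, skipping the action if either is already active.
; The roll branch checks the player's CanAttack and a close-roll chance but is disabled by a constant false, so the Dummy always attacks.
; An unreferenced Should Dodge macro rolls against a chance, prints a debug result and uses a DoOnce with delayed reset as a cooldown.
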(event EventReceiveExecuteAI
  (params (OwnerController :type AI%20Controller%20Object%20Reference) (ControlledPawn :type Pawn%20Object%20Reference))
  (bind _asdummy (Utilities|Casting|CastToDummy ControlledPawn)
    (:then
      (if (or (Variables|/Game/Character/Blueprints/Dummy.Dummy_C|Getattack _asdummy) (Variables|/Game/Character/Blueprints/Dummy.Dummy_C|GetRoll _asdummy))
        (AI|BehaviorTree|FinishExecute true)
        (else
          (if (Math|Boolean|ANDBoolean (not (Variables|/Game/Character/Blueprints/ThirdPersonCharacter.ThirdPersonCharacter_C|GetCanAttack (Variables|/Game/Character/Blueprints/Dummy.Dummy_C|GetPlayer _asdummy))) (<= (Variables|/Game/Character/Blueprints/Dummy.Dummy_C|Get2 _asdummy) (Variables|/Game/Character/Blueprints/Dummy.Dummy_C|GetCloseRollChance _asdummy)) false)
            (Default|RollEvent _asdummy)
            (else
              (Default|AttackEvent _asdummy)))
          (AI|BehaviorTree|FinishExecute true))))
    (:CastFailed
      (AI|BehaviorTree|FinishExecute false))))
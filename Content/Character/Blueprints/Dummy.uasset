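; Dummy is an AI melee combat character that spawns a sword, manages health and stamina, and ragdolls on death.
; AI perception collects players, and Tick picks the closest, updates its visibility flag and turns the status widget toward the local player's camera.
; Attack and roll events spend stamina, reroll random values and set action flags.
; When the closest player attacks, a random check can cancel the dummy's attack into a roll.
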(event OnSeePawn(PawnSensing)
  (params (Pawn :type Pawn%20Object%20Reference)))

(event OnTargetPerceptionUpdated(AIPerception)
  (params (Actor :type Actor%20Object%20Reference) (Stimulus :type AI%20Stimulus%20Structure))
  (bind _asthird_person_character (Utilities|Casting|CastToThirdPersonCharacter Actor))
  (Utilities|Array|AddUnique (Variables|Default|GetPlayers) _asthird_person_character))

(event Custom|Take%20Damage
  (params (DMG :type Float%20%28single-precision%29))
  ;[1 1 1] Take Damage
  (bind _output_get (Variables|Gameplay|SetHealth (- (Variables|Gameplay|GetHealth) DMG)))
  (if (<= _output_get 0.0)
    (CallFunction|Die)
    (elif (< (Variables|Default|GetStamina) 5e+01)
      (Variables|Default|SetStamina (+ (Variables|Default|GetStamina) 1e+01)))))

(event Custom|ClearHits
  (Default|ClearHits (Variables|Default|GetSword))
  (Variables|Default|SetdmgStart false))

(event Custom|Die
  (bind _mesh (Variables|Character|GetMesh))
  (bind _mesh_2 (Variables|Character|GetMesh))
  (Class|SkeletalMeshComponent|SetAllBodiesSimulatePhysics _mesh_2 true)
  (Physics|SetSimulatePhysics _mesh_2 true)
  (Class|PrimitiveComponent|WakeAllRigidBodies _mesh_2)
  (Rendering|SetVisibility (Variables|Default|GetWidget) false false)
  (Collision|SetCollisionResponsetoAllChannels (Variables|Collision|GetCapsuleComponent) "ECR_Ignore")
  (Collision|SetCollisionResponsetoAllChannels _mesh "ECR_Ignore")
  (Collision|SetCollisionResponsetoChannel _mesh "ECC_WorldStatic" "ECR_Block")
  (Collision|SetCollisionResponsetoChannel _mesh "ECC_WorldDynamic" "ECR_Block"))

(event Custom|CancelAttack
  (bind _closest_player (Variables|Default|GetClosest%20Player))
  (if (Utilities|IsValid _closest_player)
    (if (Math|Boolean|ANDBoolean (Variables|/Game/Character/Blueprints/ThirdPersonCharacter.ThirdPersonCharacter_C|GetAttacking _closest_player) (Variables|Default|Getattack) (<= (Variables|Default|Get1) (Variables|Default|GetAttackCancelChance)) (> (Variables|Default|GetStamina) 0.0))
      (CallFunction|RollEvent)
      (Variables|Default|Setattack false))))

(event Custom|AttackEvent
  (bind _returnvalue (Math|Random|RandomFloat))
  (if (> (Variables|Default|GetStamina) 2e+01)
    (Variables|Default|SetStamina (- (Variables|Default|GetStamina) 2e+01))
    (bind _output_get (Variables|Default|Set1 _returnvalue))
    (bind _output_get_2 (Variables|Default|Set2 _returnvalue))
    (bind _output_get_3 (Variables|Default|Set3 _returnvalue))
    (Variables|Default|Setattack true)))

(event Custom|RollEvent
  (bind _returnvalue (Math|Random|RandomFloat))
  (if (> (Variables|Default|GetStamina) 1e+01)
    (Variables|Default|SetStamina (- (Variables|Default|GetStamina) 1e+01))
    (bind _output_get (Variables|Default|Set1 _returnvalue))
    (bind _output_get_2 (Variables|Default|Set2 _returnvalue))
    (bind _output_get_3 (Variables|Default|Set3 _returnvalue))
    (Variables|Default|SetRoll true)))

(event Custom|Sense
  (bind _returnvalue (Transformation|GetActorLocation))
  (bind _players (Variables|Default|GetPlayers))
  (bind _output (Utilities|Array|Get(acopy) _players))
  (if (Utilities|IsValid _output)
    (Variables|Default|SetClosest%20Player _output)
    (for _array_element _players
      (if (< (Math|Vector|Distance(Vector) (Transformation|GetActorLocation _array_element) _returnvalue) (Math|Vector|Distance(Vector) _returnvalue (Transformation|GetActorLocation (Variables|Default|GetClosest%20Player))))
        (Variables|Default|SetClosest%20Player _array_element)))
    (if (Utilities|IsValid (Variables|Default|GetClosest%20Player))
      (if (Utilities|Array|ContainsItem (Class|AIPerceptionComponent|GetKnownPerceivedActors (Variables|Default|GetAIPerception) "/Script/AIModule.AISense_Sight") (Variables|Default|GetClosest%20Player))
        (Variables|Default|SetCanSeePlayer true)
        (else
          (Variables|Default|SetCanSeePlayer false :!label _label)))
      (else
        (goto _label)))))

(event EventBeginPlay
  (bind _returnvalue (Game|SpawnActorfromClass "/Game/CloseCombat/Weapon/Swords/SwordTest/Meshes/DummySword.DummySword_C" (Math|Transform|MakeTransform "0, 0, 0" "0, 0, 0" "1,1,1") "Undefined" 0 0))
  (Transformation|AttachComponentToComponent _returnvalue (Variables|Character|GetMesh) "Socket_Weapon" "SnapToTarget" "SnapToTarget" "SnapToTarget" true)
  (bind _output_get (Variables|Default|SetSword _returnvalue))
  (Variables|/Game/CloseCombat/Weapon/Swords/SwordTest/Meshes/DummySword.DummySword_C|SetDamage _output_get (Variables|Default|GetDamage))
  (Variables|/Game/CloseCombat/Weapon/Swords/SwordTest/Meshes/DummySword.DummySword_C|SetOwningPlayer _returnvalue self)
  (CallFunction|AttackEvent)
  (Variables|Gameplay|SetHealth (Variables|Gameplay|GetMaxHealth)))

(event Collision|EventActorBeginOverlap
  (params (OtherActor :type Actor%20Object%20Reference)))

(event EventTick
  (params (DeltaSeconds :type Float%20%28single-precision%29))
  (bind _returnvalue (Game|GetPlayerCharacter 0))
  (bind _widget (Variables|Default|GetWidget))
  ;[1 1 1] Widget Rotation
  (Utilities|FlowControl|Sequence
    (:then_0
      (if (Utilities|IsValid _returnvalue)
        (bind _asthird_person_character (Utilities|Casting|CastToThirdPersonCharacter _returnvalue))
        (Transformation|SetWorldRotation _widget (Math|Rotator|FindLookatRotation (Transformation|GetWorldLocation _widget) (Transformation|GetWorldLocation (Variables|/Game/Character/Blueprints/ThirdPersonCharacter.ThirdPersonCharacter_C|GetFollowCamera _asthird_person_character))) false false)
        (Transformation|SetWorldRotation (Variables|Default|GetArrow1) (Math|Rotator|FindLookatRotation (Transformation|GetWorldLocation _widget) (Transformation|GetWorldLocation (Variables|/Game/Character/Blueprints/ThirdPersonCharacter.ThirdPersonCharacter_C|GetFollowCamera _asthird_person_character))) false false)
        (bind _asname (Utilities|Casting|CastToName (UserInterface|GetWidget (Variables|Default|GetWidget))))
        (Progress|SetPercent (Variables|/Game/GUI/Name.Name_C|GetProgressBar_0 _asname) (/ (Variables|Gameplay|GetHealth) (Variables|Gameplay|GetMaxHealth)))
        (Progress|SetPercent (Variables|/Game/GUI/Name.Name_C|GetProgressBar _asname) (/ (Variables|Default|GetStamina) 1e+02))))
    (:then_1
      (CallFunction|CancelAttack))
    (:then_2
      (CallFunction|Sense))
    (:then_3
      (if (< (Variables|Default|GetStamina) 1e+02)
        (Utilities|FlowControl|Delay 0.1)
        (Variables|Default|SetStamina (+ (Variables|Default|GetStamina) 0.2))))))

(fn ConstructionScript)